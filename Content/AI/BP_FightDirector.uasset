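; BP_FightDirector is a fight director that staggers enemy attacks by choosing one enemy at a time on a looping timer.
; At BeginPlay it gives each enemy in EnemyList a random grade and a debug widget component showing it.
; Each tick of the timer orders the highest-graded enemy's AI_Enemy controller to attack, then re-rolls that grade and updates its widget.
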(event `self.ReceiveBeginPlay`
  (for _array_element (`self.EnemyList`)
    (`self.Add Debug Widgets` (`self.EnemyGrading`) _array_element _array_element _array_element _array_element _array_element))
  (`KismetSystemLibrary.K2_SetTimerDelegate` (delegate `TriggerAttack`) 4.0 true))

(event `TriggerAttack`
  (bind (_loc_highestvalue1 _loc_highestratedai1) (`self.FindHighestGrade`))
  (bind _asai_enemy (cast `/Game/AI/AI_Enemy` (`AIBlueprintHelperLibrary.GetAIController` _loc_highestratedai1)))
  (`/Game/AI/AI_Enemy.AI_Attack` _asai_enemy)
  (`BlueprintMapLibrary.Map_Add` (`self.EnemyGrading`) _loc_highestratedai1 (`KismetMathLibrary.RandomFloatInRange` 1.0 5.0))
  (`self.UpdateDebugInstance` _loc_highestratedai1))

(fn `Add Debug Widgets`
  (params (TargetMap :type "Map of /Game/AI/BP_EnemyAI Object Reference to Float (double-precision) (by ref)") (Key :type "/Game/AI/BP_EnemyAI Object Reference (by ref)") (EnemyInstance :type "/Game/AI/BP_EnemyAI Object Reference") (Key2 :type "/Game/AI/BP_EnemyAI Object Reference (by ref)") (self2 :type "Actor Object Reference") (Key3 :type "/Game/AI/BP_EnemyAI Object Reference (by ref)"))
  (locals (Loc_Widget :type "/Game/AI/W_DebugEnemyAI Object Reference"))
  (`BlueprintMapLibrary.Map_Add` TargetMap Key (`KismetMathLibrary.RandomFloatInRange` 1.0 5.0))
  (bind _returnvalue (`|CreateWidget` "/Game/AI/W_DebugEnemyAI.W_DebugEnemyAI_C" null EnemyInstance (`BlueprintMapLibrary.Map_Find` (`self.EnemyGrading`) Key2)))
  (set `local.Loc_Widget` _returnvalue)
  (`BlueprintMapLibrary.Map_Add` (`self.EnemyWidgets`) Key3 _returnvalue)
  (bind _returnvalue_2 (`AddComponent|NODE_AddWidgetComponent-0` :`self` self2))
  (`WidgetComponent.SetWidget` _returnvalue_2 (`local.Loc_Widget`)))

(fn `FindHighestGrade`
  (returns (Loc_highestValue1 :type "Float (double-precision)") (Loc_HighestRatedAI1 :type "/Game/AI/BP_EnemyAI Object Reference"))
  (locals (Loc_highestValue :type "Float (double-precision)") (Loc_HighestRatedAI :type "/Game/AI/BP_EnemyAI Object Reference"))
  (bind _keys (`BlueprintMapLibrary.Map_Keys` (`self.EnemyGrading`)))
  (for _array_element _keys
    (bind _value (`BlueprintMapLibrary.Map_Find` (`self.EnemyGrading`) _array_element))
    (if (> _value (`local.Loc_highestValue`))
      (set `local.Loc_highestValue` _value)
      (set `local.Loc_HighestRatedAI` _array_element)))
  (return (`local.Loc_highestValue`) (`local.Loc_HighestRatedAI`)))

(fn `UpdateDebugInstance`
  (params (EnemyInstance :type "/Game/AI/BP_EnemyAI Object Reference"))
  (set `/Game/AI/W_DebugEnemyAI.FightingGrade` (`BlueprintMapLibrary.Map_Find` (`self.EnemyGrading`) EnemyInstance) (`BlueprintMapLibrary.Map_Find` (`self.EnemyWidgets`) EnemyInstance)))

(fn `UserConstructionScript`)