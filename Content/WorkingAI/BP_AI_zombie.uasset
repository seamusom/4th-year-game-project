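; Zombie AI character that wanders slowly until it sees or hears the player, then plays audio and speeds up.
; Begin play seeds the Blackboard with start location, wander range and default behavior through a BBData helper, leaving movement decisions outside this graph.
; Pawn sensing stores the first detected enemy in the Blackboard and fires PlayerSpotted.
; Damage drains health, then triggers Died, ragdolls the mesh and destroys the actor after a delay.
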(event `self.ReceiveBeginPlay`
  (bind (_returnvalue _returnvalue2) (`self.BB_Data` "StartLocation"))
  (bind (_returnvalue_2 _returnvalue2_2) (`self.BB_Data` "WanderingRange"))
  (bind (_returnvalue_3 _returnvalue2_3) (`self.BB_Data` "DefaultBehavior"))
  (set `self.Start_Location` (`self.K2_GetActorLocation`))
  (`BlackboardComponent.SetValueAsFloat` _returnvalue_2 _returnvalue2_2 (`self.Max_WanderDistance`))
  (`BlackboardComponent.SetValueAsEnum` _returnvalue_3 _returnvalue2_3 (`self.Default_Behavior`))
  (`BlackboardComponent.SetValueAsVector` _returnvalue _returnvalue2 (`self.Start_Location`))
  (set `CharacterMovementComponent.MaxWalkSpeed` 100.0 (`self.CharacterMovement`)))

(event `self.ReceiveAnyDamage`
  (params (Damage :type "Float (single-precision)") (DamageType :type "DamageType Object Reference") (InstigatedBy :type "Controller Object Reference") (DamageCauser :type "Actor Object Reference"))
  (bind _mesh (`self.Mesh`))
  (set `self.Health` (- (`self.Health`) Damage))
  (if (< (`self.Health`) 1.0)
    (`/Engine/EditorBlueprintResources/StandardMacros.DoOnce` false
      (:`Completed`
        (`self.died`)
        (`ActorComponent.Deactivate` (`self.Audio`))
        (`PrimitiveComponent.SetCollisionEnabled` _mesh "PhysicsOnly")
        (`PrimitiveComponent.SetSimulatePhysics` _mesh true)
        (`PrimitiveComponent.SetCollisionEnabled` (`self.CapsuleComponent`) "NoCollision")
        (`ActorComponent.Deactivate` (`self.Audio`))
        (`KismetSystemLibrary.Delay` 5.0)
        (`self.K2_DestroyActor`)))))

(event `self.PawnSensing.OnSeePawn`
  (params (Pawn :type "Pawn Object Reference"))
  (bind (_returnvalue _returnvalue2) (`self.BB_Data` "Enemy"))
  (if (== (`GameplayStatics.GetPlayerCharacter` 0) Pawn)
    (`AudioComponent.Play` (`self.Audio`) 0.0 :!label _label)
    (`self.EnemyPawn`
      (:`then`)
      (:`else`
        (bind _output_get (set `self.EnemyPawn` Pawn))
        (`BlackboardComponent.SetValueAsObject` _returnvalue _returnvalue2 _output_get)
        (set `CharacterMovementComponent.MaxWalkSpeed` 250.0 (`self.CharacterMovement`))
        (`self.Player spotted`)))))

(event `self.PawnSensing.OnHearNoise`
  (params (Instigator :type "Pawn Object Reference") (Location :type "Vector Structure (by ref)") (Volume :type "Float (single-precision)"))
  (cast `/Game/Character/BP_FPSCharacter` Instigator)
  (goto _label))

(fn `BB_Data`
  (params (KeyName :type Name))
  (returns (ReturnValue :type "BlackboardComponent Object Reference") (ReturnValue2 :type Name))
  (return (`AIBlueprintHelperLibrary.GetBlackboard` (`AIBlueprintHelperLibrary.GetAIController` self)) (`KismetSystemLibrary.MakeLiteralName` KeyName)))

(fn `UserConstructionScript`)