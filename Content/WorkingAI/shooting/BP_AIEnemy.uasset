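; BP_AIEnemy is a stationary-logic shooter enemy that attacks the FPS player character on sight.
; When PawnSensing sees a BP_FPSCharacter, it snaps to face it and, if able, spawns a fireball with a firing sound at Spawnloc.
; A CanAttack flag and short Delay throttle the fire rate.
; Any damage reduces Health, destroying the actor once it drops below one.
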(event `self.PawnSensing.OnSeePawn`
  (params (Pawn :type "Pawn Object Reference"))
  (bind _spawnloc (`self.spawnloc`))
  (bind _asbp_fpscharacter (cast `/Game/Character/BP_FPSCharacter` Pawn))
  (`self.K2_SetActorRotation` (`KismetMathLibrary.FindRelativeLookAtRotation` (`KismetMathLibrary.Conv_VectorToTransform` (`self.K2_GetActorLocation`)) (`self.K2_GetActorLocation` _asbp_fpscharacter)))
  (if (`self.CanAttack?`)
    (`|SpawnActorFromClass` "/Game/WorkingAI/shooting/FireBall_2.FireBall_2_C" (`SceneComponent.K2_GetComponentToWorld` _spawnloc) "Undefined" "OverrideRootScale" null null)
    (`GameplayStatics.SpawnSoundAttached` "/Game/WorkingAI/shooting/shotgun-firing-4-6746.shotgun-firing-4-6746" _spawnloc "None" (0.0 0.0 0.0) (struct) "KeepRelativeOffset" false 1.0 1.0 0.0 null null)
    (set `self.CanAttack?` false)
    (`KismetSystemLibrary.Delay` 0.6)
    (set `self.CanAttack?` true)))

(event `self.ReceiveAnyDamage`
  (params (Damage :type "Float (single-precision)") (DamageType :type "DamageType Object Reference") (InstigatedBy :type "Controller Object Reference") (DamageCauser :type "Actor Object Reference"))
  (set `self.Health` (- (`self.Health`) Damage))
  (if (< (`self.Health`) 1.0)
    (`self.K2_DestroyActor`)))

(fn `UserConstructionScript`)