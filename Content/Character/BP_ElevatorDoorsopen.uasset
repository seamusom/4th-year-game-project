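; BP_ElevatorDoorsopen is an elevator door actor that animates its doors and moves the game on to another level.
; Any actor overlap starts a sequence in which, after a short delay, two timelines lerp the right and left door transforms between their start and end values.
; A parallel, longer delay then opens the level named by NextLevel, with no check on which actor triggered it.
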(event `self.ReceiveActorBeginOverlap`
  (params (OtherActor :type "Actor Object Reference"))
  (`|ExecutionSequence`
    (:`then_0`
      (`KismetSystemLibrary.Delay` 0.5)
      (bind (_direction _newtrack_1) (`Timeline|Timeline_0`)
        (:`Update`
          (`SceneComponent.K2_SetRelativeTransform` (`self.right door`) (`KismetMathLibrary.TLerp` (`self.Start right door`) (`self.end right door`) _newtrack_1) false false))))
    (:`then_1`
      (`KismetSystemLibrary.Delay` 0.5)
      (bind (_direction_2 _newtrack_1_2) (`Timeline|Timeline_1`)
        (:`Update`
          (`SceneComponent.K2_SetRelativeTransform` (`self.left door`) (`KismetMathLibrary.TLerp` (`self.Start left door`) (`self.End left door`) _newtrack_1_2) false false))))
    (:`then_2`
      (`KismetSystemLibrary.Delay` 5.0)
      (`GameplayStatics.OpenLevel` (`self.Next level`)))))

(fn `UserConstructionScript`)