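; BP_ElevatorDoors is an elevator door Blueprint that opens or closes its two door meshes automatically a few seconds after BeginPlay.
; A Sequence starts two delayed timelines in parallel, one per door.
; Each timeline's track blends that door between stored start and end transforms with LerpTransform and applies it as a relative transform, without sweep.
; It has no trigger, reverse or construction logic, so the motion plays once.
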(event `self.ReceiveBeginPlay`
  (`|ExecutionSequence`
    (:`then_0`
      (`KismetSystemLibrary.Delay` 3.0)
      (bind (_direction _newtrack_1) (`Timeline|Door`)
        (:`Update`
          (`SceneComponent.K2_SetRelativeTransform` (`self.right door`) (`KismetMathLibrary.TLerp` (`self.Start right door`) (`self.end right door`) _newtrack_1) false false))))
    (:`then_1`
      (`KismetSystemLibrary.Delay` 3.0)
      (bind (_direction_2 _newtrack_1_2) (`Timeline|Timeline_0`)
        (:`Update`
          (`SceneComponent.K2_SetRelativeTransform` (`self.left door`) (`KismetMathLibrary.TLerp` (`self.Start left door`) (`self.End left door`) _newtrack_1_2) false false))))))

(fn `UserConstructionScript`)